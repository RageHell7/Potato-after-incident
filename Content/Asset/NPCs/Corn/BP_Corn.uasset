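; BP_Corn is a corn NPC Blueprint that shows its dialogue one line at a time in an on-screen widget.
; Each CornDialogue event advances an index into the Yap array and writes that line to a WB_CornDialogues widget, creating it if none is valid.
; Once the lines run out, it removes the widget, clears the reference and resets the index.
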(event `/Game/Asset/NPCs/Corn/BPI_CornDialogue.CornDialogue`
  (`/Engine/EditorBlueprintResources/StandardMacros.IncrementInt` (`self.TalkIndex`)
    (:`  `
      (if (< (`self.TalkIndex`) (`KismetArrayLibrary.Array_Length` (`self.yap`)))
        (`self.DialogueCorn`
          (:`then`
            _)
          (:`else`
            (bind _returnvalue (`|CreateWidget` "/Game/Asset/NPCs/Corn/WB_CornDialogues.WB_CornDialogues_C"))
            (bind _output_get (set `self.DialogueCorn` _returnvalue))
            (`UserWidget.AddToViewport` _output_get 0)))
        (`TextBlock.SetText` (`/Game/Asset/NPCs/Corn/WB_CornDialogues.TextBlock_35` (`self.DialogueCorn`)) (`KismetTextLibrary.Conv_StringToText` (`|GetArrayItem` (`self.yap`) (`self.TalkIndex`))))
        (else
          (`Widget.RemoveFromParent` (`self.DialogueCorn`))
          (set `self.TalkIndex` -1)
          (set `self.DialogueCorn` null))))))

(fn `UserConstructionScript`)