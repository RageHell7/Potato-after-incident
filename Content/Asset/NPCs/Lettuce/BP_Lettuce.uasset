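; BP_Lettuce is a lettuce NPC that shows dialogue to the player one line at a time.
; Each LettuceDialogue call advances an index through the Yap array, creating the WB_LettuceDialogue widget if needed and updating its text.
; After the last line it removes the widget, resets the index and sets the BP_Potat player's movement mode back to Walking.
; Taking damage only prints an "ouchie" message with the amount.
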(event `/Game/Asset/NPCs/Lettuce/BPI_Lettuce.LettuceDialogue`
  (`/Engine/EditorBlueprintResources/StandardMacros.IncrementInt` (`self.TalkIndex`)
    (:`  `
      (if (< (`self.TalkIndex`) (`KismetArrayLibrary.Array_Length` (`self.yap`)))
        (`self.LettuceDialogueUI`
          (:`then`
            _)
          (:`else`
            (bind _returnvalue (`|CreateWidget` "/Game/Asset/NPCs/Lettuce/WB_LettuceDialogue.WB_LettuceDialogue_C"))
            (bind _output_get (set `self.LettuceDialogueUI` _returnvalue))
            (`UserWidget.AddToViewport` _output_get 0)
            (`UserWidget.AddToViewport` (`self.LettuceDialogueUI`) 0)))
        (`TextBlock.SetText` (`/Game/Asset/NPCs/Lettuce/WB_LettuceDialogue.Lettuce` (`self.LettuceDialogueUI`)) (`KismetTextLibrary.Conv_StringToText` (`|GetArrayItem` (`self.yap`) (`self.TalkIndex`))))
        (else
          (`Widget.RemoveFromParent` (`self.LettuceDialogueUI`))
          (set `self.TalkIndex` -1)
          (set `self.LettuceDialogueUI` null)
          (bind _asbp_potat (cast `/Game/Asset/Potat/BP_Potat` (`GameplayStatics.GetPlayerCharacter` 0)))
          (`CharacterMovementComponent.SetMovementMode` (`Character.CharacterMovement` _asbp_potat) "MOVE_Walking" 0))))))

(event `self.ReceiveAnyDamage`
  (params (Damage :type "Float (single-precision)") (DamageType :type "DamageType Object Reference") (InstigatedBy :type "Controller Object Reference") (DamageCauser :type "Actor Object Reference"))
  ;[0.2554 0.7586 1] event take damage
  (`KismetSystemLibrary.PrintString` (`KismetStringLibrary.Concat_StrStr` "ouchie" (`KismetStringLibrary.Conv_DoubleToString` Damage))))

(fn `UserConstructionScript`)