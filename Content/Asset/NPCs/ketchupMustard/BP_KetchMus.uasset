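; BP_KetchMus is an NPC Blueprint that plays a linear, line-by-line dialogue with the player.
; Each KetchMusDialogue event advances TalkIndex through the Yap array, lazily creating a WB_KetchMusDialogue widget and setting its text to the current line.
; After the last line it removes the widget, resets the index and sets the BP_Potat player's movement mode back to Walking.
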(event `/Game/Asset/NPCs/ketchupMustard/BPI_KetchMus.KetchMus Dialogue`
  (`/Engine/EditorBlueprintResources/StandardMacros.IncrementInt` (`self.TalkIndex`)
    (:`  `
      (if (< (`self.TalkIndex`) (`KismetArrayLibrary.Array_Length` (`self.yap`)))
        (`self.WB KetchMus Dialogue`
          (:`then`
            _)
          (:`else`
            (bind _returnvalue (`|CreateWidget` "/Game/Asset/NPCs/ketchupMustard/WB_KetchMusDialogue.WB_KetchMusDialogue_C"))
            (bind _output_get (set `self.WB KetchMus Dialogue` _returnvalue))
            (`UserWidget.AddToViewport` _output_get 0)
            (`UserWidget.AddToViewport` (`self.WB KetchMus Dialogue`) 0)))
        (`TextBlock.SetText` (`/Game/Asset/NPCs/ketchupMustard/WB_KetchMusDialogue.KetchMus` (`self.WB KetchMus Dialogue`)) (`KismetTextLibrary.Conv_StringToText` (`|GetArrayItem` (`self.yap`) (`self.TalkIndex`))))
        (else
          (`Widget.RemoveFromParent` (`self.WB KetchMus Dialogue`))
          (set `self.TalkIndex` -1)
          (set `self.WB KetchMus Dialogue` null)
          (bind _asbp_potat (cast `/Game/Asset/Potat/BP_Potat` (`GameplayStatics.GetPlayerCharacter` 0)))
          (`CharacterMovementComponent.SetMovementMode` (`Character.CharacterMovement` _asbp_potat) "MOVE_Walking" 0))))))

(fn `UserConstructionScript`)