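; BP_Camphor is an NPC Blueprint that steps the player through Camphor's dialogue lines on screen.
; Each CamphorDialogue call advances TalkIndex through the Yap array, creating a WB_CamphorDialogue widget if none exists and setting its text to the current line.
; After the last line it removes the widget, resets the index and sets the BP_Potat player's movement mode back to Walking.
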(event `/Game/Asset/NPCs/Camphor/BPI_CamphorDialogue.CamphorDialogue`
  (`/Engine/EditorBlueprintResources/StandardMacros.IncrementInt` (`self.Talk Index`)
    (:`  `
      (if (< (`self.Talk Index`) (`KismetArrayLibrary.Array_Length` (`self.yap`)))
        (`self.Dialogue UI`
          (:`then`
            _)
          (:`else`
            (bind _returnvalue (`|CreateWidget` "/Game/Asset/NPCs/Camphor/WB_CamphorDialogue.WB_CamphorDialogue_C"))
            (bind _output_get (set `self.Dialogue UI` _returnvalue))
            (`UserWidget.AddToViewport` _output_get 0)
            (`UserWidget.AddToViewport` (`self.Dialogue UI`) 0)))
        (`TextBlock.SetText` (`/Game/Asset/NPCs/Camphor/WB_CamphorDialogue.camphodialogue` (`self.Dialogue UI`)) (`KismetTextLibrary.Conv_StringToText` (`|GetArrayItem` (`self.yap`) (`self.Talk Index`))))
        (else
          (`Widget.RemoveFromParent` (`self.Dialogue UI`))
          (set `self.Talk Index` -1)
          (set `self.Dialogue UI` null)
          (bind _asbp_potat (cast `/Game/Asset/Potat/BP_Potat` (`GameplayStatics.GetPlayerCharacter` 0)))
          (`CharacterMovementComponent.SetMovementMode` (`Character.CharacterMovement` _asbp_potat) "MOVE_Walking" 0))))))

(fn `UserConstructionScript`)