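; BP_Spider is a spider NPC Blueprint that shows dialogue to the player through a WB_TomatoDialogues widget.
; Each TomatoDialogue call advances an index into the Yap lines, creating the widget if needed and setting its text.
; Past the last line, it removes the widget, resets the index and restores BP_Potat's movement to Walking.
; AnyDamage is empty, with enemy health-bar update logic left disconnected.
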(event `self.TomatoDialogue`
  (`/Engine/EditorBlueprintResources/StandardMacros.IncrementInt` (`self.TalkIndex`)
    (:`  `
      (if (< (`self.TalkIndex`) (`KismetArrayLibrary.Array_Length` (`self.yap`)))
        (`self.DialogueUI`
          (:`then`
            _)
          (:`else`
            (bind _returnvalue (`|CreateWidget` "/Game/Asset/NPCs/Tomato/WB_TomatoDialogues.WB_TomatoDialogues_C"))
            (bind _output_get (set `self.DialogueUI` _returnvalue))
            (`UserWidget.AddToViewport` (`self.DialogueUI`) 0)
            (`UserWidget.AddToViewport` _output_get 0)))
        (`TextBlock.SetText` (`/Game/Asset/NPCs/Tomato/WB_TomatoDialogues.TextBlock_34` (`self.DialogueUI`)) (`KismetTextLibrary.Conv_StringToText` (`|GetArrayItem` (`self.yap`) (`self.TalkIndex`))))
        (else
          (`Widget.RemoveFromParent` (`self.DialogueUI`))
          (set `self.TalkIndex` -1)
          (set `self.DialogueUI` null)
          (bind _asbp_potat (cast `/Game/Asset/Potat/BP_Potat` (`GameplayStatics.GetPlayerCharacter` 0)))
          (`CharacterMovementComponent.SetMovementMode` (`Character.CharacterMovement` _asbp_potat) "MOVE_Walking" 0))))))

(event `self.ReceiveAnyDamage`
  (params (Damage :type "Float (single-precision)") (DamageType :type "DamageType Object Reference") (InstigatedBy :type "Controller Object Reference") (DamageCauser :type "Actor Object Reference"))
  ;[0.2542 0.7605 1] event take damage
)

(fn `UserConstructionScript`)