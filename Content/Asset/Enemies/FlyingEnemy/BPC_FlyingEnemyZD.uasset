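; Flying enemy that runs a behavior tree and continuously fires short-lived bullets at the player.
; Tick aims an arrow at the player and starts a self-repeating delayed spawn loop through DoOnce, currently not gated by sight.
; While stationary it advances a looping spline location; two forward traces set SplineOverlap, cleared when the player is far.
; AI perception sight updates CanSee and the TargetActor blackboard key.
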(event `ShootPlayer`
  (bind (_returnvalue_location _returnvalue_rotation) (`KismetMathLibrary.BreakTransform` (`SceneComponent.K2_GetComponentToWorld` (`self.Arrow1`))))
  (`/Engine/EditorBlueprintResources/StandardMacros.DoOnce` false
    (:`Completed`
      ;[1 1 1] Shooting Aimmed at Player
      (bind _returnvalue (`|SpawnActorFromClass` "/Game/Asset/Enemies/FlyingEnemy/BPA_Bullets.BPA_Bullets_C" (`KismetMathLibrary.MakeTransform` _returnvalue_location _returnvalue_rotation) "Undefined" "MultiplyWithRoot" null null :!label _label))
      (`self.SetLifeSpan` _returnvalue 2.0)
      (`KismetSystemLibrary.Delay` 0.5)
      (goto _label))))

(event `self.AIPerception.OnTargetPerceptionUpdated`
  (params (Actor :type "Actor Object Reference") (Stimulus :type "AIStimulus Structure"))
  (`self.AI Sight` Actor Stimulus))

(event `self.ReceiveBeginPlay`
  (`AIController.RunBehaviorTree` (`AIBlueprintHelperLibrary.GetAIController` self) "/Game/Asset/Enemies/FlyingEnemy/BT_FlyingEnemyZD.BT_FlyingEnemyZD"))

(event `self.ReceiveTick`
  (params (DeltaSeconds :type "Float (single-precision)"))
  (bind _arrow1 (`self.Arrow1`))
  (bind _arrow3 (`self.Arrow3`))
  (bind _arrow4 (`self.Arrow4`))
  (bind _returnvalue (`SceneComponent.K2_GetComponentLocation` _arrow3))
  (bind _returnvalue_2 (`SceneComponent.K2_GetComponentLocation` _arrow4))
  (`|ExecutionSequence`
    (:`then_0`
      (`self.ShootPlayer`)
      (`SceneComponent.K2_SetWorldRotation` _arrow1 (`KismetMathLibrary.FindLookAtRotation` (`SceneComponent.K2_GetComponentLocation` _arrow1) (`SceneComponent.K2_GetComponentLocation` (`Actor.RootComponent` (`GameplayStatics.GetPlayerPawn` 0)))) true false)
      (if (== (`self.GetVelocity`) (0.0 0.0 0.0))
        (set `self.Spline Distance` (+ (`self.Spline Distance`) 0.0017))
        (if (>= (`self.Spline Distance`) 1.0)
          (set `self.Spline Distance` 0.0))
        (set `self.Spline Location` (`SplineComponent.GetLocationAtDistanceAlongSpline` (`self.Spline`) (`KismetMathLibrary.Lerp` 0.0 (`SplineComponent.GetSplineLength` (`self.Spline`)) (`self.Spline Distance`)) "World"))))
    (:`then_1`
      (bind _outhit (`KismetSystemLibrary.LineTraceSingle` :`Start` _returnvalue :`End` (+ _returnvalue (* (`SceneComponent.GetForwardVector` _arrow3) 350.0)) :`TraceChannel` "TraceTypeQuery1" :`DrawDebugType` "ForDuration"))
      (if (`GameplayStatics.BreakHitResult` _outhit)
        (set `self.SplineOverlap` true)))
    (:`then_2`
      (bind _outhit_2 (`KismetSystemLibrary.LineTraceSingle` :`Start` _returnvalue_2 :`End` (+ _returnvalue_2 (* (`SceneComponent.GetForwardVector` _arrow4) 350.0)) :`TraceChannel` "TraceTypeQuery1" :`DrawDebugType` "ForDuration"))
      (if (`GameplayStatics.BreakHitResult` _outhit_2)
        (set `self.SplineOverlap` true)))
    (:`then_3`
      (if (>= (`self.GetDistanceTo` (`GameplayStatics.GetPlayerCharacter` 0)) 900.0)
        (set `self.SplineOverlap` false)))))

(fn `AI Sight`
  (params (Actor :type "Actor Object Reference") (Stimulus :type "AIStimulus Structure"))
  (bind _returnvalue (`GameplayStatics.GetPlayerCharacter` 0))
  (bind (_stimulus_age _stimulus_expirationage _stimulus_strength _stimulus_stimuluslocation _stimulus_receiverlocation _stimulus_tag _stimulus_bsuccessfullysensed) (break `AIStimulus` (`local.Stimulus`)))
  (bind _returnvalue_2 (`AIPerceptionSystem.GetSenseClassForStimulus` Stimulus))
  (if (== _returnvalue_2 "/Script/AIModule.AISense_Sight")
    (if (== Actor _returnvalue)
      (`self.SetCanSee` _stimulus_bsuccessfullysensed)
      (`BlackboardComponent.SetValueAsObject` (`AIBlueprintHelperLibrary.GetBlackboard` null) "TargetActor" (select `bool` _stimulus_bsuccessfullysensed :`true` _returnvalue :!type "Object Object Reference"))
      (if _stimulus_bsuccessfullysensed
        (return)
        (else
          (`BlackboardComponent.SetValueAsVector` (`AIBlueprintHelperLibrary.GetBlackboard` null) "TargetActor" _stimulus_stimuluslocation)))
      (else
        (return)))
    (else
      (return))))

(fn `SetCanSee`
  (params (Condition :type Boolean))
  (if Condition
    (set `self.Can See?` true)
    (return)
    (else
      (set `self.Can See?` false)
      (return))))

(fn `UserConstructionScript`)