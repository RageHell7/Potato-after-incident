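; Flying enemy character that runs BT_FlyingEnemy and feeds player sight updates to the Blackboard's TargetActor key.
; Tick turns Arrow1 toward the player and, while the enemy is stationary, advances a looping SplineLocation along its spline.
; ShootPlayer spawns short-lived BPA_Bullets at Arrow1 using ShootingStar rotations in a delayed repeating loop.
; An aimed-at-player firing loop is present but disconnected.
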(event `self.AIPerception.OnTargetPerceptionUpdated`
  (params (Actor :type "Actor Object Reference") (Stimulus :type "AIStimulus Structure"))
  (`self.AISight` Actor Stimulus))

(event `self.ReceiveBeginPlay`
  (`AIController.RunBehaviorTree` (`AIBlueprintHelperLibrary.GetAIController` self) "/Game/Asset/Enemies/FlyingEnemy/BT_FlyingEnemy.BT_FlyingEnemy"))

(event `self.ReceiveTick`
  (params (DeltaSeconds :type "Float (single-precision)"))
  (bind _arrow1 (`self.Arrow1`))
  (`SceneComponent.K2_SetWorldRotation` _arrow1 (`KismetMathLibrary.FindLookAtRotation` (`SceneComponent.K2_GetComponentLocation` _arrow1) (`SceneComponent.K2_GetComponentLocation` (`Actor.RootComponent` (`GameplayStatics.GetPlayerPawn` 0)))) true false)
  (if (== (`self.GetVelocity`) (0.0 0.0 0.0))
    (set `self.SplineDistance` (+ (`self.SplineDistance`) 0.002))
    (if (>= (`self.SplineDistance`) 1.0)
      (set `self.SplineDistance` 0.0))
    (set `self.SplineLocation` (`SplineComponent.GetLocationAtDistanceAlongSpline` (`self.Spline`) (`KismetMathLibrary.Lerp` 0.0 (`SplineComponent.GetSplineLength` (`self.Spline`)) (`self.SplineDistance`)) "World"))))

(event `ShootPlayer`
  (bind (_returnvalue_location _returnvalue_rotation) (`KismetMathLibrary.BreakTransform` (`SceneComponent.K2_GetComponentToWorld` (`self.Arrow1`))))
  (if true
    ;[1 1 1] Shooting in star
    (for _array_element (`self.ShootingStar`) :!label _label
      (bind _returnvalue (`|SpawnActorFromClass` "/Game/Asset/Enemies/FlyingEnemy/BPA_Bullets.BPA_Bullets_C" (`KismetMathLibrary.MakeTransform` _returnvalue_location _array_element) "Undefined" "MultiplyWithRoot" null null))
      (`self.SetLifeSpan` _returnvalue 2.0)
      (`KismetSystemLibrary.Delay` 1.5)
      (goto _label))))

(fn `AISight`
  (params (Actor :type "Actor Object Reference") (Stimulus :type "AIStimulus Structure"))
  (bind _returnvalue (`GameplayStatics.GetPlayerCharacter` 0))
  (bind (_stimulus_age _stimulus_expirationage _stimulus_strength _stimulus_stimuluslocation _stimulus_receiverlocation _stimulus_tag _stimulus_bsuccessfullysensed) (break `AIStimulus` (`local.Stimulus`)))
  (bind _returnvalue_2 (`AIPerceptionSystem.GetSenseClassForStimulus` Stimulus))
  (if (== _returnvalue_2 "/Script/AIModule.AISenseConfig_Sight")
    (if (== Actor _returnvalue)
      (`BlackboardComponent.SetValueAsObject` (`AIBlueprintHelperLibrary.GetBlackboard` null) "TargetActor" (select `bool` _stimulus_bsuccessfullysensed :`true` _returnvalue :!type "Object Object Reference"))
      (if _stimulus_bsuccessfullysensed
        (return)
        (else
          (`BlackboardComponent.SetValueAsVector` (`AIBlueprintHelperLibrary.GetBlackboard` null) "TargetActor" _stimulus_stimuluslocation)))
      (else
        (return)))
    (else
      (return))))

(fn `UserConstructionScript`)