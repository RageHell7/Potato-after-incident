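; BP_MarianoYap is a Blueprint that shows lines of boss dialogue for Mariano through an on-screen widget.
; The Mariano event lazily creates WB_MarianoDialogue, then loops over the Yap array with a long Delay between lines and removes the widget once the index reaches the array length.
; TalkIndex increments both before display and after the delay, so only every other entry is shown.
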(event `/Game/Asset/Enemies/Boss/Dialogue/BPI_BossDialogue.Mariano`
  (if (< (`self.TalkIndex`) (`KismetArrayLibrary.Array_Length` (`self.yap`))) :!label _label
    (`/Engine/EditorBlueprintResources/StandardMacros.IncrementInt` (`self.TalkIndex`)
      (:`  `
        (`self.MarianoDialogue`
          (:`then`
            _)
          (:`else`
            (bind _returnvalue (`|CreateWidget` "/Game/Asset/Enemies/Boss/Dialogue/WB_MarianoDialogue.WB_MarianoDialogue_C"))
            (bind _output_get (set `self.MarianoDialogue` _returnvalue))
            (`UserWidget.AddToViewport` _output_get 0)))
        (`TextBlock.SetText` (`/Game/Asset/Enemies/Boss/Dialogue/WB_MarianoDialogue.Mariano` (`self.MarianoDialogue`)) (`KismetTextLibrary.Conv_StringToText` (`|GetArrayItem` (`self.yap`) (`self.TalkIndex`))))
        (`KismetSystemLibrary.Delay` 500.0)
        (`/Engine/EditorBlueprintResources/StandardMacros.IncrementInt` (`self.TalkIndex`)
          (:`  `
            (goto _label)))))
    (else
      (`Widget.RemoveFromParent` (`self.MarianoDialogue`)))))

(fn `UserConstructionScript`)