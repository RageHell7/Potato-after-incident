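; BP_Pepper is a boss enemy that continuously fires pepper flake projectiles at the player.
; Tick rotates Arrow1 to face the player pawn and calls ShootPlayer, where a DoOnce starts a self-repeating Delay loop.
; Each pass spawns a short-lived BPA_PepperFlake at the arrow's location and rotation.
; The shooting condition is hardcoded true, so the DoOnce reset branch never runs.
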(event `self.ReceiveBeginPlay`)

(event `self.ReceiveTick`
  (params (DeltaSeconds :type "Float (single-precision)"))
  (bind _arrow1 (`self.Arrow1`))
  (`|ExecutionSequence`
    (:`then_0`
      (`self.ShootPlayer`)
      (`SceneComponent.K2_SetWorldRotation` _arrow1 (`KismetMathLibrary.FindLookAtRotation` (`SceneComponent.K2_GetComponentLocation` _arrow1) (`SceneComponent.K2_GetComponentLocation` (`Actor.RootComponent` (`GameplayStatics.GetPlayerPawn` 0)))) true false))))

(event `ShootPlayer`
  (bind (_returnvalue_location _returnvalue_rotation) (`KismetMathLibrary.BreakTransform` (`SceneComponent.K2_GetComponentToWorld` (`self.Arrow1`))))
  (if true
    (`/Engine/EditorBlueprintResources/StandardMacros.DoOnce` false :!label _label
      (:`Completed`
        ;[1 1 1] Shooting Aimmed at Player
        (bind _returnvalue (`|SpawnActorFromClass` "/Game/Asset/Enemies/Boss/BPA_PepperFlake.BPA_PepperFlake_C" (`KismetMathLibrary.MakeTransform` _returnvalue_location _returnvalue_rotation) "Undefined" "MultiplyWithRoot" null null :!label _label_2))
        (`self.SetLifeSpan` _returnvalue 2.0)
        (`KismetSystemLibrary.Delay` 0.5)
        (goto _label_2)))
    (else
      (goto _label :!via `Reset`))))

(fn `UserConstructionScript`)