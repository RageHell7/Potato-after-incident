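; Boss controller that defines three health-based phases, each spawning a pair of boss actors at left and right hand locations.
; High health spawns the hands, the middle band swaps them for Salt and Pepper, and the low band for ChilliHand and Chilli.
; Tick runs these checks through a DoOnce with no visible reset, so they evaluate only once.
; Any box overlap subtracts a large fixed chunk of Health and prints debug text.
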(event `self.ReceiveTick`
  (params (DeltaSeconds :type "Float (single-precision)"))
  (`/Engine/EditorBlueprintResources/StandardMacros.DoOnce` false
    (:`Completed`
      (`|ExecutionSequence`
        (:`then_0`
          (if (> (`self.Health`) 400)
            (bind _returnvalue (`|SpawnActorFromClass` "/Game/Asset/Enemies/Boss/BP_LeftHand.BP_LeftHand_C" (`KismetMathLibrary.MakeTransform` (`self.LeftHandLocation`) (struct :`Yaw` 90.0)) "Undefined" "MultiplyWithRoot" null null))
            (bind _returnvalue_2 (`|SpawnActorFromClass` "/Game/Asset/Enemies/Boss/BP_RightHand.BP_RightHand_C" (`KismetMathLibrary.MakeTransform` (`self.RightHandLocation`) (struct :`Yaw` 90.0)) "Undefined" "MultiplyWithRoot" null null))))
        (:`then_1`
          (if (and (< (`self.Health`) 400) (> (`self.Health`) 200))
            (`self.K2_DestroyActor` _returnvalue)
            (`self.K2_DestroyActor` _returnvalue_2)
            (bind _returnvalue_3 (`|SpawnActorFromClass` "/Game/Asset/Enemies/Boss/BP_Salt.BP_Salt_C" (`KismetMathLibrary.MakeTransform` (`self.LeftHandLocation`) (struct :`Yaw` 90.0)) "Undefined" "MultiplyWithRoot" null null))
            (bind _returnvalue_4 (`|SpawnActorFromClass` "/Game/Asset/Enemies/Boss/BP_Pepper.BP_Pepper_C" (`KismetMathLibrary.MakeTransform` (`self.RightHandLocation`) (struct :`Yaw` 90.0)) "Undefined" "MultiplyWithRoot" null null))))
        (:`then_2`
          (if (and (< (`self.Health`) 200) (> (`self.Health`) 0))
            (`self.K2_DestroyActor` _returnvalue_3)
            (`self.K2_DestroyActor` _returnvalue_4)
            (`|SpawnActorFromClass` "/Game/Asset/Enemies/Boss/BP_ChilliHand.BP_ChilliHand_C" (`KismetMathLibrary.MakeTransform` (`self.LeftHandLocation`) (struct :`Yaw` 90.0)) "Undefined" "MultiplyWithRoot" null null)
            (`|SpawnActorFromClass` "/Game/Asset/Enemies/StatusEffectEnemy/Level1/BP_Chilli.BP_Chilli_C" (`KismetMathLibrary.MakeTransform` (`self.RightHandLocation`) (struct :`Yaw` 90.0)) "Undefined" "MultiplyWithRoot" null null)))))))

(event `self.Box.OnComponentBeginOverlap`
  (params (OverlappedComponent :type "PrimitiveComponent Object Reference") (OtherActor :type "Actor Object Reference") (OtherComp :type "PrimitiveComponent Object Reference") (OtherBodyIndex :type Integer) (bFromSweep :type Boolean) (SweepResult :type "HitResult Structure (by ref)"))
  (`KismetSystemLibrary.PrintString` "overlap")
  (bind _output_get (set `self.Health` (- (`self.Health`) 201)))
  (`KismetSystemLibrary.PrintString` (`KismetStringLibrary.Conv_IntToString` _output_get)))

(fn `UserConstructionScript`)