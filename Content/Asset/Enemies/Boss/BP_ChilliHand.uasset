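; A boss enemy hand that fires repeating star-shaped volleys of BP_Chilli projectiles.
; Tick turns Arrow1 toward the player and calls ShootPlayer, whose DoOnce starts the firing loop only once because its branch is always true.
; Each volley spawns short-lived chillies at the arrow's location using ShootingStar rotations rather than its aim.
; A Delay wired back into the ForEach repeats the volley every ten seconds.
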(event `self.ReceiveTick`
  (params (DeltaSeconds :type "Float (single-precision)"))
  (bind _arrow1 (`self.Arrow1`))
  (`|ExecutionSequence`
    (:`then_0`
      (`self.ShootPlayer`)
      (`SceneComponent.K2_SetWorldRotation` _arrow1 (`KismetMathLibrary.FindLookAtRotation` (`SceneComponent.K2_GetComponentLocation` _arrow1) (`SceneComponent.K2_GetComponentLocation` (`Actor.RootComponent` (`GameplayStatics.GetPlayerPawn` 0)))) true false))))

(event `ShootPlayer`
  (bind _returnvalue_location (`KismetMathLibrary.BreakTransform` (`SceneComponent.K2_GetComponentToWorld` (`self.Arrow1`))))
  (if true
    (`/Engine/EditorBlueprintResources/StandardMacros.DoOnce` false :!label _label
      (:`Completed`
        ;[1 1 1] Shooting in star
        (for _array_element (`self.ShootingStar`) :!label _label_2
          (bind _returnvalue (`|SpawnActorFromClass` "/Game/Asset/Enemies/StatusEffectEnemy/Level1/BP_Chilli.BP_Chilli_C" (`KismetMathLibrary.MakeTransform` _returnvalue_location _array_element) "Undefined" "MultiplyWithRoot" null null))
          (`self.SetLifeSpan` _returnvalue 2.0)
          (`KismetSystemLibrary.Delay` 10.0)
          (goto _label_2))))
    (else
      (goto _label :!via `Reset`))))

(fn `UserConstructionScript`)