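; BP_LeftHand is a boss enemy Blueprint for the left hand that feeds player sightings into its AI Blackboard.
; AIPerception target updates go to AISight, which ignores everything except sight stimuli from player character 0.
; Sensing the player stores it as the TargetActor object.
; Losing sight clears that object, then writes the stimulus location as a vector to the same TargetActor key name.
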(event `self.AIPerception.OnTargetPerceptionUpdated`
  (params (Actor :type "Actor Object Reference") (Stimulus :type "AIStimulus Structure"))
  (`self.AI Sight` Actor Stimulus))

(fn `AI Sight`
  (params (Actor :type "Actor Object Reference") (Stimulus :type "AIStimulus Structure"))
  (bind (_stimulus_age _stimulus_expirationage _stimulus_strength _stimulus_stimuluslocation _stimulus_receiverlocation _stimulus_tag _stimulus_bsuccessfullysensed) (break `AIStimulus` (`local.Stimulus`)))
  (bind _returnvalue (`AIPerceptionSystem.GetSenseClassForStimulus` Stimulus))
  (if (== _returnvalue "/Script/AIModule.AISense_Sight")
    (if (== Actor (`GameplayStatics.GetPlayerCharacter` 0))
      (`BlackboardComponent.SetValueAsObject` (`AIBlueprintHelperLibrary.GetBlackboard` null) "TargetActor" (select `bool` _stimulus_bsuccessfullysensed :`true` Actor :!type "Object Object Reference"))
      (if _stimulus_bsuccessfullysensed
        (return)
        (else
          (`BlackboardComponent.SetValueAsVector` (`AIBlueprintHelperLibrary.GetBlackboard` null) "TargetActor" _stimulus_stimuluslocation)))
      (else
        (return)))
    (else
      (return))))

(fn `UserConstructionScript`)