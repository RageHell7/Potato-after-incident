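; BP_EnemyBase is an enemy Blueprint, named as a base, that tracks health and shows it on a health bar widget.
; Tick casts the WCHB component's widget to WB_HealthBarEnemy and sets its progress bar from HealthBase as a percentage.
; AnyDamage prints a debug string and stores health minus damage divided by 100, a scaling that Tick applies again.
; No death handling is present.
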(event `self.ReceiveTick`
  (params (DeltaSeconds :type "Float (single-precision)"))
  (bind _aswb_health_bar_enemy (cast `/Game/Asset/UI/WB_HealthBarEnemy` (`WidgetComponent.GetWidget` (`self.WC_HB`))))
  (`ProgressBar.SetPercent` (`/Game/Asset/UI/WB_HealthBarEnemy.HBprogressbar` _aswb_health_bar_enemy) (/ (`self.HealthBase`) 100.0)))

(event `self.ReceiveAnyDamage`
  (params (Damage :type "Float (single-precision)") (DamageType :type "DamageType Object Reference") (InstigatedBy :type "Controller Object Reference") (DamageCauser :type "Actor Object Reference"))
  ;[0.2542 0.7605 1] event take damage
  (`KismetSystemLibrary.PrintString` "hurtenemy")
  (set `self.HealthBase` (/ (- (`self.HealthBase`) Damage) 100.0)))

(fn `UserConstructionScript`)