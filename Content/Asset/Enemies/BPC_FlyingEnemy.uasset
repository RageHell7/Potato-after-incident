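; Flying enemy character that runs the BT_FlyingEnemy behavior tree and repeatedly fires bullets in a star pattern.
; Tick advances a looping fraction along a spline by a fixed per-frame step to update SplineLocation, and turns an arrow toward the player.
; ShootPlayer spawns short-lived BPA_Bullets at the arrow for each ShootingStar rotation, repeating through a delay.
; An alternate player-aimed firing loop is present but disconnected.
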(event `self.ReceiveBeginPlay`
  (`AIController.RunBehaviorTree` (`AIBlueprintHelperLibrary.GetAIController` self) "/Game/Asset/Enemies/BT_FlyingEnemy.BT_FlyingEnemy")
  (`self.ShootPlayer`))

(event `self.ReceiveTick`
  (params (DeltaSeconds :type "Float (single-precision)"))
  (bind _arrow1 (`self.Arrow1`))
  (set `self.SplineDistance` (+ (`self.SplineDistance`) 0.007))
  (if (>= (`self.SplineDistance`) 1.0)
    (set `self.SplineDistance` 0.0))
  (set `self.SplineLocation` (`SplineComponent.GetLocationAtDistanceAlongSpline` (`self.Spline`) (`KismetMathLibrary.Lerp` 0.0 (`SplineComponent.GetSplineLength` (`self.Spline`)) (`self.SplineDistance`)) "World"))
  (`SceneComponent.K2_SetWorldRotation` _arrow1 (`KismetMathLibrary.FindLookAtRotation` (`SceneComponent.K2_GetComponentLocation` _arrow1) (`SceneComponent.K2_GetComponentLocation` (`Actor.RootComponent` (`GameplayStatics.GetPlayerPawn` 0)))) false false))

(event `ShootPlayer`
  (bind (_returnvalue_location _returnvalue_rotation) (`KismetMathLibrary.BreakTransform` (`SceneComponent.K2_GetComponentToWorld` (`self.Arrow1`))))
  ;[1 1 1] Shooting in star
  (for _array_element (`self.ShootingStar`) :!label _label
    (bind _returnvalue (`|SpawnActorFromClass` "/Game/Asset/Enemies/BPA_Bullets.BPA_Bullets_C" (`KismetMathLibrary.MakeTransform` _returnvalue_location _array_element) "Undefined" "MultiplyWithRoot" null null))
    (`self.SetLifeSpan` _returnvalue 2.0)
    (`KismetSystemLibrary.Delay` 1.5)
    (goto _label)))

(fn `UserConstructionScript`)