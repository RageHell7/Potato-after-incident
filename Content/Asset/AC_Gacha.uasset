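; Gacha component (by its AC_ name) that rolls a weighted random index when the attack input, right-click input or 1 key fires.
; SumValues totals the WeightValues array, and a random float up to that total goes to DetermineIndex.
; DetermineIndex walks the cumulative weights and returns the first index whose running sum reaches the roll.
; The GachaResult lookup by that index is left unused, so the roll has no further effect.
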(event `self.ReceiveBeginPlay`)

(event `EnhancedInput|/Game/ThirdPerson/Input/Actions/IA_ATTACK`
  (params (ActionValue :type Boolean) (ElapsedSeconds :type "Float (double-precision)") (TriggeredSeconds :type "Float (double-precision)") (InputAction :type "InputAction Object Reference" :default "/Game/ThirdPerson/Input/Actions/IA_ATTACK.IA_ATTACK"))
  (:`Started`
    (bind _sumofvalues (`self.SumValues` :!label _label))
    (bind _indexwon (`self.DetermineIndex` (`KismetMathLibrary.RandomFloatInRange` 0.0 _sumofvalues)))))

(event `Key|One`
  (params (Key :type "Key Structure"))
  (:`Pressed`
    (goto _label)))

(event `EnhancedInput|/Game/ThirdPerson/Input/Actions/IA_RightClick`
  (params (ActionValue :type Boolean) (ElapsedSeconds :type "Float (double-precision)") (TriggeredSeconds :type "Float (double-precision)") (InputAction :type "InputAction Object Reference" :default "/Game/ThirdPerson/Input/Actions/IA_RightClick.IA_RightClick"))
  (:`Started`
    (goto _label)))

(fn `DetermineIndex`
  (params (RandomValue :type "Float (double-precision)"))
  (returns (IndexWon :type Integer))
  (locals (LocalSum :type "Float (double-precision)"))
  (for (_array_element _array_index) (`self.WeightValues`)
    (bind _output_get (set `local.LocalSum` (+ _array_element (`local.LocalSum`))))
    (if (>= _output_get RandomValue)
      (break)))
  (return _array_index))

(fn `SumValues`
  (returns (SumOfValues :type "Float (double-precision)"))
  (locals (LocalSum :type "Float (double-precision)"))
  (for _array_element (`self.WeightValues`)
    (set `local.LocalSum` (+ _array_element (`local.LocalSum`))))
  (return (`local.LocalSum`)))