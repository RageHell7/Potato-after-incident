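; BP_Potat is the side-scrolling player character, with double jump, velocity-based dashes, melee and a pause menu.
; Landing resets the double jump and the DoOnce gates that limit dashes, while jump and attack events drive animation node jumps.
; Overlapping "Ladder"-tagged actors switches movement to Flying for climbing.
; Interact sends interface messages to overlapping actors, disabling movement for Tomato, Corn and Lettuce dialogue.
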(event `KelarLompat`
  ;[1 0.151 0.2435] Jump Animation
  (set `self.JumpingCondition?` false))

(event `self.OnJumped`
  ;[1 0.151 0.2435] Jump Animation
  (set `self.JumpingCondition?` true :!label _label)
  (set `self.IsClimbing?` false)
  (`PaperZDAnimInstance.JumpToNode` (`PaperZDAnimationComponent.AnimInstance` (`self.AnimationComponent`)) "JumpActivated" "None"))

(event `self.OnWalkingOffLedge`
  (params (PreviousFloorImpactNormal :type "Vector Structure (by ref)") (PreviousFloorContactNormal :type "Vector Structure (by ref)") (PreviousLocation :type "Vector Structure (by ref)") (TimeDelta :type "Float (single-precision)"))
  ;[1 0.151 0.2435] Jump Animation
  (goto _label))

(event `self.ReceiveBeginPlay`
  ;[1 1 1] AC Gacha and Input Mapping
  (`AddComponent|NODE_AddAC_Gacha-0`)
  (message `EnhancedInputSubsystemInterface.AddMappingContext` (pcsubsystem `EnhancedInputLocalPlayerSubsystem` (`GameplayStatics.GetPlayerController` 0)) "/Game/ThirdPerson/Input/IMC_Default.IMC_Default" 0 (struct)))

(event `EnhancedInput|/Game/ThirdPerson/Input/Actions/IA_Jump`
  (params (ActionValue :type Boolean) (ElapsedSeconds :type "Float (double-precision)") (TriggeredSeconds :type "Float (double-precision)") (InputAction :type "InputAction Object Reference" :default "/Game/ThirdPerson/Input/Actions/IA_Jump.IA_Jump"))
  ;[0.749 0.309 0.1194] Jump & Double Jump
)

(event `self.ReceiveTick`
  (params (DeltaSeconds :type "Float (single-precision)")))

(event `InputAxis|MoveRight`
  (params (AxisValue :type "Float (single-precision)"))
  (`|ExecutionSequence`
    (:`then_0`
      (`self.AddMovementInput` (0.0 1.0 0.0) AxisValue))
    (:`then_1`
      (if (== AxisValue 1.0)
        (set `self.Idle` true)
        (elif (== AxisValue -1.0)
          (set `self.Idle` false))))))

(event `EnhancedInput|/Game/ThirdPerson/Input/Actions/IA_Pause`
  (params (ActionValue :type Boolean) (ElapsedSeconds :type "Float (double-precision)") (TriggeredSeconds :type "Float (double-precision)") (InputAction :type "InputAction Object Reference" :default "/Game/ThirdPerson/Input/Actions/IA_Pause.IA_Pause"))
  (bind _returnvalue (`GameplayStatics.GetPlayerController` 0))
  (:`Started`
    (if (not (`self.IsPauseOpen?`))
      (set `self.IsPauseOpen?` true)
      (bind _returnvalue_2 (`|CreateWidget` "/Game/Asset/UI/WB_game.WB_game_C" _returnvalue))
      (bind _output_get (set `self.pauseMenuWidget` _returnvalue_2))
      (`UserWidget.AddToViewport` _output_get 0)
      (`Widget.SetVisibility` (`/Game/Asset/UI/WB_game.GUI` (`self.pauseMenuWidget`)) "Hidden")
      (`Widget.SetVisibility` (`/Game/Asset/UI/WB_game.mainmenu` (`self.pauseMenuWidget`)) "Hidden")
      (`Widget.SetVisibility` (`/Game/Asset/UI/WB_game.pausemenu` (`self.pauseMenuWidget`)) "Visible")
      (`WidgetBlueprintLibrary.SetInputMode_GameAndUIEx` _returnvalue (`self.pauseMenuWidget`))
      (set `PlayerController.bShowMouseCursor` true (`GameplayStatics.GetPlayerController` 0))
      (`GameplayStatics.SetGamePaused` true)
      (else
        (set `self.IsPauseOpen?` false)
        (`Widget.RemoveFromParent` (`self.pauseMenuWidget`))
        (`GameplayStatics.SetGamePaused` false)
        (`WidgetBlueprintLibrary.SetInputMode_GameOnly` null)
        (set `PlayerController.bShowMouseCursor` false (`GameplayStatics.GetPlayerController` 0))))))

(event `EnhancedInput|/Game/ThirdPerson/Input/Actions/IA_Dash`
  (params (ActionValue :type Boolean) (ElapsedSeconds :type "Float (double-precision)") (TriggeredSeconds :type "Float (double-precision)") (InputAction :type "InputAction Object Reference" :default "/Game/ThirdPerson/Input/Actions/IA_Dash.IA_Dash"))
  ;[1 0.8148 0.2928] Dashing
)

(event `InputAction|MeleeAttack`
  (params (Key :type "Key Structure"))
  ;[0.2156 0.04054 0.02293] Melee Attack
  (:`Pressed`
    (if (not (`self.Attacking`))
      (set `self.Attacking` true)
      (`PaperZDAnimInstance.JumpToNode` (`PaperZDAnimationComponent.AnimInstance` (`self.AnimationComponent`)) "Attack" "None")
      (set `self.Attacking` false))))

(event `EnhancedInput|/Game/ThirdPerson/Input/Actions/IA_Jump`
  (params (ActionValue :type Boolean) (ElapsedSeconds :type "Float (double-precision)") (TriggeredSeconds :type "Float (double-precision)") (InputAction :type "InputAction Object Reference" :default "/Game/ThirdPerson/Input/Actions/IA_Jump.IA_Jump"))
  (:`Started`
    (set `self.JumpingCondition?` true)
    (`self.Jump`)
    (if (and (`NavMovementComponent.IsFalling` (`self.CharacterMovement`)) (`self.Can Double Jump`))
      (`KismetSystemLibrary.PrintString` "Hello")
      (set `self.Can Double Jump` false)
      (set `self.JumpingCondition?` false)
      (`self.LaunchCharacter` (`KismetMathLibrary.MakeVector` 0.0 0.0 (* (`CharacterMovementComponent.JumpZVelocity` (`self.CharacterMovement`)) 1.7)) false true)))
  (:`Completed`
    (`self.StopJumping`)))

(event `self.OnLanded`
  (params (Hit :type "HitResult Structure (by ref)"))
  (bind (_returnvalue_x _returnvalue_y) (`KismetMathLibrary.BreakVector` (`self.GetVelocity`)))
  (bind (_returnvalue_x_2 _returnvalue_y_2) (`KismetMathLibrary.BreakVector` (`self.GetVelocity`)))
  (bind (_returnvalue_x_3 _returnvalue_y_3) (`KismetMathLibrary.BreakVector` (* (`KismetMathLibrary.MakeVector` _returnvalue_x _returnvalue_y) 1.5)))
  (bind (_returnvalue_x_4 _returnvalue_y_4) (`KismetMathLibrary.BreakVector` (* (`KismetMathLibrary.MakeVector` _returnvalue_x_2 _returnvalue_y_2) 1.5)))
  (set `self.Can Double Jump` true)
  (set `self.IsDashing` false)
  (`|ExecutionSequence`
    (:`then_0`
      (goto _label_3 :!via `Reset`))
    (:`then_1`
      (goto _label_4 :!via `Reset`))))

(event `NAIK TANGGGA TOLOL`
  ;[0.6875 0.7948 0.1968] Climbing
  (set `self.IsClimbing?` true :!label _label_2)
  (`CharacterMovementComponent.SetMovementMode` (`self.CharacterMovement`) "MOVE_Flying" 0)
  (`self.AddMovementInput` (0.0 0.0 1.0) (`.Y` (`KismetMathLibrary.BreakVector2D` (stale `EnhancedInput|/Game/ThirdPerson/Input/Actions/IA_Move` ActionValue)))))

(event `EnhancedInput|/Game/ThirdPerson/Input/Actions/IA_Move`
  (params (ActionValue :type "Vector2D Structure") (ElapsedSeconds :type "Float (double-precision)") (TriggeredSeconds :type "Float (double-precision)") (InputAction :type "InputAction Object Reference" :default "/Game/ThirdPerson/Input/Actions/IA_Move.IA_Move"))
  ;[0.6875 0.7948 0.1968] Climbing
  (:`Triggered`
    (if (and (!= ActionValue_Y 0.0) (`self.IsOnLadder?`))
      (goto _label_2))))

(event `EnhancedInput|/Game/ThirdPerson/Input/Actions/IA_Dash`
  (params (ActionValue :type Boolean) (ElapsedSeconds :type "Float (double-precision)") (TriggeredSeconds :type "Float (double-precision)") (InputAction :type "InputAction Object Reference" :default "/Game/ThirdPerson/Input/Actions/IA_Dash.IA_Dash"))
  (bind (_returnvalue_x _returnvalue_y) (`KismetMathLibrary.BreakVector` (`self.GetVelocity`)))
  (bind (_returnvalue_x_2 _returnvalue_y_2) (`KismetMathLibrary.BreakVector` (`self.GetVelocity`)))
  (bind (_returnvalue_x_3 _returnvalue_y_3) (`KismetMathLibrary.BreakVector` (`self.GetVelocity`)))
  (bind (_returnvalue_x_4 _returnvalue_y_4) (`KismetMathLibrary.BreakVector` (* (`KismetMathLibrary.MakeVector` _returnvalue_x_2 _returnvalue_y_2) 5.0)))
  (bind (_returnvalue_x_5 _returnvalue_y_5) (`KismetMathLibrary.BreakVector` (* (`KismetMathLibrary.MakeVector` _returnvalue_x _returnvalue_y) 1.5)))
  (bind (_returnvalue_x_6 _returnvalue_y_6) (`KismetMathLibrary.BreakVector` (* (`KismetMathLibrary.MakeVector` _returnvalue_x_3 _returnvalue_y_3) 1.5)))
  (:`Started`
    (if (`self.IsDashing`)
      _
      (elif (`self.JumpingCondition?`)
        (`/Engine/EditorBlueprintResources/StandardMacros.DoOnce` false :!label _label_3
          (:`Completed`
            (set `self.IsDashing` true)
            (`self.LaunchCharacter` (`KismetMathLibrary.MakeVector` _returnvalue_x_5 _returnvalue_y_5))
            (set `self.IsDashing` false)
            (set `self.JumpingCondition?` true)))
        (elif (`self.Can Double Jump`)
          (set `self.IsDashing` true)
          (`self.LaunchCharacter` (`KismetMathLibrary.MakeVector` _returnvalue_x_4 _returnvalue_y_4))
          (`KismetSystemLibrary.Delay` 0.2)
          (set `self.IsDashing` false)
          (else
            (`/Engine/EditorBlueprintResources/StandardMacros.DoOnce` false :!label _label_4
              (:`Completed`
                (set `self.IsDashing` true)
                (`self.LaunchCharacter` (`KismetMathLibrary.MakeVector` _returnvalue_x_6 _returnvalue_y_6))
                (`KismetSystemLibrary.Delay` 0.2)
                (set `self.IsDashing` false)))))))))

(event `EnhancedInput|/Game/ThirdPerson/Input/Actions/IA_Interact`
  (params (ActionValue :type Boolean) (ElapsedSeconds :type "Float (double-precision)") (TriggeredSeconds :type "Float (double-precision)") (InputAction :type "InputAction Object Reference" :default "/Game/ThirdPerson/Input/Actions/IA_Interact.IA_Interact"))
  ;[1 1 1] Interact
  (:`Started`
    (for _array_element (`self.GetOverlappingActors` null)
      (if (`KismetSystemLibrary.DoesImplementInterface` _array_element "/Game/Asset/BI_InteractAction.BI_InteractAction_C")
        (message `/Game/Asset/BI_InteractAction.Interact` _array_element self)
        (break)))))

(event `self.CapsuleComponent.OnComponentBeginOverlap`
  (params (OverlappedComponent :type "PrimitiveComponent Object Reference") (OtherActor :type "Actor Object Reference") (OtherComp :type "PrimitiveComponent Object Reference") (OtherBodyIndex :type Integer) (bFromSweep :type Boolean) (SweepResult :type "HitResult Structure (by ref)"))
  ;[0.6875 0.7948 0.1968] Climbing
  (if (`self.ActorHasTag` OtherActor "Ladder")
    (set `self.IsOnLadder?` true)
    (`self.NAIK TANGGGA TOLOL`)))

(event `self.CapsuleComponent.OnComponentEndOverlap`
  (params (OverlappedComponent :type "PrimitiveComponent Object Reference") (OtherActor :type "Actor Object Reference") (OtherComp :type "PrimitiveComponent Object Reference") (OtherBodyIndex :type Integer))
  ;[0.6875 0.7948 0.1968] Climbing
  (if (`self.ActorHasTag` OtherActor "Ladder")
    (set `self.IsOnLadder?` false)
    (set `self.IsClimbing?` false)
    (`CharacterMovementComponent.SetMovementMode` (`self.CharacterMovement`) "MOVE_Walking" 0)))

(event `EnhancedInput|/Game/ThirdPerson/Input/Actions/IA_Interact`
  (params (ActionValue :type Boolean) (ElapsedSeconds :type "Float (double-precision)") (TriggeredSeconds :type "Float (double-precision)") (InputAction :type "InputAction Object Reference" :default "/Game/ThirdPerson/Input/Actions/IA_Interact.IA_Interact"))
  (:`Started`
    (for _array_element (`self.GetOverlappingActors` "/Game/Asset/NPCs/Tomato/BP_Tomato.BP_Tomato_C")
      (if (`KismetSystemLibrary.DoesImplementInterface` _array_element "/Game/Asset/NPCs/Tomato/BPI_Tomato.BPI_Tomato_C")
        (`CharacterMovementComponent.DisableMovement` (`self.CharacterMovement`))
        (message `/Game/Asset/NPCs/Tomato/BPI_Tomato.TomatoDialogue` _array_element)))))

(event `EnhancedInput|/Game/ThirdPerson/Input/Actions/IA_Interact`
  (params (ActionValue :type Boolean) (ElapsedSeconds :type "Float (double-precision)") (TriggeredSeconds :type "Float (double-precision)") (InputAction :type "InputAction Object Reference" :default "/Game/ThirdPerson/Input/Actions/IA_Interact.IA_Interact"))
  (:`Started`
    (for _array_element (`self.GetOverlappingActors` "/Game/Asset/NPCs/Corn/BP_Corn.BP_Corn_C")
      (if (`KismetSystemLibrary.DoesImplementInterface` _array_element "/Game/Asset/NPCs/Corn/BPI_CornDialogue.BPI_CornDialogue_C")
        (`CharacterMovementComponent.DisableMovement` (`self.CharacterMovement`))
        (message `/Game/Asset/NPCs/Corn/BPI_CornDialogue.CornDialogue` _array_element)))))

(event `EnhancedInput|/Game/ThirdPerson/Input/Actions/IA_Interact`
  (params (ActionValue :type Boolean) (ElapsedSeconds :type "Float (double-precision)") (TriggeredSeconds :type "Float (double-precision)") (InputAction :type "InputAction Object Reference" :default "/Game/ThirdPerson/Input/Actions/IA_Interact.IA_Interact"))
  (:`Started`
    (for _array_element (`self.GetOverlappingActors` "/Game/Asset/NPCs/Lettuce/BP_Lettuce.BP_Lettuce_C")
      (if (`KismetSystemLibrary.DoesImplementInterface` _array_element "/Game/Asset/NPCs/Lettuce/BPI_Lettuce.BPI_Lettuce_C")
        (`CharacterMovementComponent.DisableMovement` (`self.CharacterMovement`))
        (message `/Game/Asset/NPCs/Lettuce/BPI_Lettuce.LettuceDialogue` _array_element)))))

(fn `UserConstructionScript`)