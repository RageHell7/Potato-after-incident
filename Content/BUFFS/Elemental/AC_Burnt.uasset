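; AC_Burnt is an actor component that gives its owner a chance to catch fire, as an elemental burn debuff.
; On BeginPlay a weighted random roll over WeightValue picks a BuffResult flag that enables damage on Tick.
; A successful roll slows ticking to half-second intervals, attaches NS_Fire and stores it on the player's BP_Potat.
; After five seconds it destroys itself and the effect; a failed roll leaves the component idle.
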(event `self.ReceiveTick`
  (params (DeltaSeconds :type "Float (single-precision)"))
  (`|ExecutionSequence`
    (:`then_0`
      (if (`self.ActivateTick`)
        (`GameplayStatics.ApplyDamage` (`self.GetOwner`) 2.0)))))

(event `self.ReceiveBeginPlay`
  (bind _returnvalue (`self.GetOwner`))
  (bind _sumofvalue (`self.SumValue`))
  (bind _indexwon (`self.DeteminedIndex` (`KismetMathLibrary.RandomFloatInRange` 0.0 _sumofvalue)))
  (bind _output (`|GetArrayItem` (`self.BuffResult`) _indexwon))
  (set `self.ActivateTick` _output)
  (if _output
    (`KismetSystemLibrary.PrintString` "BURN!!")
    (`self.SetComponentTickInterval` 0.5)
    (`KismetSystemLibrary.PrintString` (`KismetSystemLibrary.GetDisplayName` _returnvalue))
    (bind _returnvalue_2 (`NiagaraFunctionLibrary.SpawnSystemAttached` "/Game/Asset/Enemies/StatusEffectEnemy/SFXnya/Niagara/NS_Fire.NS_Fire" (`Actor.RootComponent` _returnvalue) "None" (0.0 0.0 0.0) (struct) "KeepRelativeOffset"))
    (bind _asbp_potat (cast `/Game/Asset/Potat/BP_Potat` (`GameplayStatics.GetPlayerCharacter` 0)))
    (set `/Game/Asset/Potat/BP_Potat.JanganHapusNanti` _returnvalue_2 _asbp_potat)
    (`KismetSystemLibrary.Delay` 5.0)
    (`self.K2_DestroyComponent`)
    (`self.K2_DestroyComponent` _returnvalue_2)))

(fn `DeteminedIndex`
  (params (RandomValue :type "Float (double-precision)"))
  (returns (IndexWon :type Integer))
  (locals (LocalSum :type "Float (double-precision)"))
  (for (_array_element _array_index) (`self.WeightValue`)
    (bind _output_get (set `local.LocalSum` (+ _array_element (`local.LocalSum`))))
    (if (>= _output_get RandomValue)
      (break)))
  (return _array_index))

(fn `SumValue`
  (returns (SumOfValue :type "Float (double-precision)"))
  (locals (LocalSum :type "Float (double-precision)"))
  (for _array_element (`self.WeightValue`)
    (set `local.LocalSum` (+ _array_element (`local.LocalSum`))))
  (return (`local.LocalSum`)))