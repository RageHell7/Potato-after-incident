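; Actor component for a Frozen elemental debuff that has a weighted random chance to slow the character it is attached to.
; On BeginPlay, SumValues and DetermineIndex pick a weighted index from WeightValue, which looks up a boolean in BuffResult.
; On success it lowers the PaperZD character's walk speed and attaches a particle emitter.
; After a delay it destroys itself without restoring speed; a failed roll leaves it attached.
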(event `self.ReceiveBeginPlay`
  (bind _returnvalue (`self.GetOwner`))
  (bind _sumofvalues (`self.SumValues`))
  (bind _indexwon (`self.DetermineIndex` (`KismetMathLibrary.RandomFloatInRange` 0.0 _sumofvalues)))
  (if (`|GetArrayItem` (`self.BuffResult`) _indexwon)
    (`KismetSystemLibrary.PrintString` "FROZEN!!")
    (bind _aspaper_zdcharacter (cast `PaperZDCharacter` _returnvalue))
    (set `CharacterMovementComponent.MaxWalkSpeed` 50.0 (`Character.CharacterMovement` _aspaper_zdcharacter))
    (`GameplayStatics.SpawnEmitterAttached` "/Engine/Functions/Engine_MaterialFunctions02/ExampleContent/3dParticleOpacity_Particle.3dParticleOpacity_Particle" (`Actor.RootComponent` _returnvalue))
    (`KismetSystemLibrary.Delay` 5.0)
    (`self.K2_DestroyComponent`)))

(fn `DetermineIndex`
  (params (RandomValue :type "Float (double-precision)"))
  (returns (IndexWon :type Integer))
  (locals (LocalSum :type "Float (double-precision)"))
  (for (_array_element _array_index) (`self.WeightValue`)
    (bind _output_get (set `local.LocalSum` (+ _array_element (`local.LocalSum`))))
    (if (>= _output_get RandomValue)
      (break)))
  (return _array_index))

(fn `SumValues`
  (returns (SumOfValues :type "Float (double-precision)"))
  (locals (LocalSum :type "Float (double-precision)"))
  (for _array_element (`self.WeightValue`)
    (set `local.LocalSum` (+ _array_element (`local.LocalSum`))))
  (return (`local.LocalSum`)))