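; Actor component for a paralyze debuff that rolls on BeginPlay whether to affect its PaperZD character owner.
; The roll is a weighted random pick: SumValue totals WeightValue, and DetermineIndex finds the index whose boolean in BuffResult decides success.
; On success it stops active movement once, attaches a Niagara paralyze effect, and destroys itself after a placeholder delay.
; A failed roll does nothing and leaves the component in place.
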(event `self.ReceiveBeginPlay`
  (bind _returnvalue (`self.GetOwner`))
  (bind _sumofvalue (`self.SumValue`))
  (bind _indexwon (`self.DetermineIndex` (`KismetMathLibrary.RandomFloatInRange` 0.0 _sumofvalue)))
  (if (`|GetArrayItem` (`self.BuffResult`) _indexwon)
    (bind _aspaper_zdcharacter (cast `PaperZDCharacter` _returnvalue))
    (`KismetSystemLibrary.PrintString` "PARALYZE!")
    (`NavMovementComponent.StopActiveMovement` (`Character.CharacterMovement` _aspaper_zdcharacter))
    (`NiagaraFunctionLibrary.SpawnSystemAttached` "/Game/Asset/Enemies/StatusEffectEnemy/SFXnya/Niagara/NS_Paralyze.NS_Paralyze" (`Actor.RootComponent` _returnvalue) "None" (0.0 0.0 0.0) (struct) "KeepRelativeOffset")
    (`KismetSystemLibrary.Delay` 5.0) ; ADJUST DELAY LTR
    (`self.K2_DestroyComponent`)))

(fn `DetermineIndex`
  (params (`Random Value` :type "Float (double-precision)"))
  (returns (IndexWon :type Integer))
  (locals (LocalSum :type "Float (double-precision)"))
  (for (_array_element _array_index) (`self.WeightValue`)
    (bind _output_get (set `local.LocalSum` (+ _array_element (`local.LocalSum`))))
    (if (>= _output_get `Random Value`)
      (break)))
  (return _array_index))

(fn `SumValue`
  (returns (SumOfValue :type "Float (double-precision)"))
  (locals (LocalSum :type "Float (double-precision)"))
  (for _array_element (`self.WeightValue`)
    (set `local.LocalSum` (+ _array_element (`local.LocalSum`))))
  (return (`local.LocalSum`)))