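; BP_SpeedParticle is a speed buff actor that doubles the walk speed of the Character it is attached to, relative to a hard-coded 600 baseline.
; An actor overlap starts a short delay, then raises MaxWalkSpeed on the attach parent, regardless of which actor overlapped.
; EndPlay resets the parent to that fixed baseline, without saving the original speed.
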(event `self.ReceiveActorBeginOverlap`
  (params (OtherActor :type "Actor Object Reference"))
  (`parent.ReceiveActorBeginOverlap` OtherActor)
  (`KismetSystemLibrary.Delay` 0.2)
  (bind _ascharacter (cast `Character` (`self.GetAttachParentActor`)))
  (set `CharacterMovementComponent.MaxWalkSpeed` 1200.0 (`Character.CharacterMovement` _ascharacter)))

(event `self.ReceiveEndPlay`
  (params (EndPlayReason :type "EEndPlayReason Enum" :default "Destroyed"))
  (bind _ascharacter (cast `Character` (`self.GetAttachParentActor`)))
  (set `CharacterMovementComponent.MaxWalkSpeed` 600.0 (`Character.CharacterMovement` _ascharacter)))

(fn `UserConstructionScript`
  (`parent.UserConstructionScript`))