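; Buff pickup base actor that grants BP_Potat a random status effect on overlap, then destroys itself.
; SumValues and DetermineIndex perform a weighted random roll over WeightValues to index the Buff array.
; SwitchBuff selects whether the result sets the melee StatusEffects or the RangeStatusEffect, with debug prints.
; A DoOnce precedes the cast, so only the first overlap by any actor is processed.
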(event `self.ReceiveActorBeginOverlap`
  (params (OtherActor :type "Actor Object Reference"))
  (`/Engine/EditorBlueprintResources/StandardMacros.DoOnce` false
    (:`Completed`
      (bind _asbp_potat (cast `/Game/Asset/Potat/BP_Potat` OtherActor))
      (bind _sumofvalues (`self.SumValues`))
      (bind _indexwon (`self.DetermineIndex` (`KismetMathLibrary.RandomFloatInRange` 0.0 _sumofvalues)))
      (switch `/Game/BUFFS/Elemental/E_AssignBuffTo` (`self.SwitchBuff`)
        (:`NewEnumerator0`
          (bind _output (`|GetArrayItem` (`self.Buff`) _indexwon))
          (bind _output_get (set `/Game/Asset/Potat/BP_Potat.StatusEffects` _output _asbp_potat))
          (`KismetSystemLibrary.PrintString` (`|GetEnumeratorNameAsString` _output_get))
          (`self.K2_DestroyActor`)
          (`KismetSystemLibrary.PrintString` "destroyed"))
        (:`NewEnumerator1`
          (`KismetSystemLibrary.PrintString` "Hello")
          (bind _output_get_2 (set `/Game/Asset/Potat/BP_Potat.Range Status Effect` _output _asbp_potat))
          (`KismetSystemLibrary.PrintString` (`|GetEnumeratorNameAsString` _output_get_2))
          (`self.K2_DestroyActor`)
          (`KismetSystemLibrary.PrintString` "destroyed"))))))

(fn `DetermineIndex`
  (params (RandomValue :type "Float (double-precision)"))
  (returns (IndexWon :type Integer))
  (locals (LocalSum :type "Float (double-precision)"))
  (for (_array_element _array_index) (`self.WeightValues`)
    (bind _output_get (set `local.LocalSum` (+ _array_element (`local.LocalSum`))))
    (if (>= _output_get RandomValue)
      (break)))
  (return _array_index))

(fn `SumValues`
  (returns (SumOfValues :type "Float (double-precision)"))
  (locals (LocalSum :type "Float (double-precision)"))
  (for _array_element (`self.WeightValues`)
    (set `local.LocalSum` (+ _array_element (`local.LocalSum`))))
  (return (`local.LocalSum`)))

(fn `UserConstructionScript`
  (`parent.UserConstructionScript`))