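; BP_SpeedEffect is a buff effect actor that makes the Character it is attached to move faster for as long as the effect exists.
; Shortly after BeginPlay, it casts its attach parent to Character and raises Max Walk Speed.
; EndPlay sets that speed back to a hardcoded value rather than restoring the character's original speed.
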(event `self.ReceiveBeginPlay`
  (`KismetSystemLibrary.Delay` 0.2)
  (bind _ascharacter (cast `Character` (`self.GetAttachParentActor`)))
  (set `CharacterMovementComponent.MaxWalkSpeed` 1200.0 (`Character.CharacterMovement` _ascharacter)))

(event `self.ReceiveEndPlay`
  (params (EndPlayReason :type "EEndPlayReason Enum" :default "Destroyed"))
  (bind _ascharacter (cast `Character` (`self.GetAttachParentActor`)))
  (set `CharacterMovementComponent.MaxWalkSpeed` 600.0 (`Character.CharacterMovement` _ascharacter)))

(fn `UserConstructionScript`
  (`parent.UserConstructionScript`))